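; Player character Blueprint that manages health and owns the HUD, pause, game over and win widgets.
; BeginPlay creates all four widgets but shows only the HUD.
; AnyDamage subtracts from Vida behind a DoOnce that resets after a brief MostrarDaño flag pulse and delay, giving a short invulnerability window.
; Depleted Vida triggers EventFinalDeJuego, which, like EventGanaste, clears widgets, shows its screen with UI-only input and cursor, and pauses the game.
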(event `self.ReceiveBeginPlay`
  ;[1 1 1] Crear HUD en menu
  (bind _returnvalue (`|CreateWidget` "/Game/MiContenido/Blueprints/TheHUD.TheHUD_C"))
  (bind _output_get (set `self.MyHUD` _returnvalue))
  (`UserWidget.AddToViewport` _output_get 0)
  (bind _returnvalue_2 (`|CreateWidget` "/Game/MiContenido/Blueprints/MenuPausa.MenuPausa_C"))
  (set `self.Pausa` _returnvalue_2)
  (bind _returnvalue_3 (`|CreateWidget` "/Game/MiContenido/Blueprints/GameOver.GameOver_C"))
  (set `self.GameOver` _returnvalue_3)
  (bind _returnvalue_4 (`|CreateWidget` "/Game/MiContenido/Blueprints/Ganaste.Ganaste_C"))
  (set `self.Ganaste` _returnvalue_4))

(event `EventFinalDeJuego`
  (bind _returnvalue (`GameplayStatics.GetPlayerController` 0))
  (bind _gameover (`self.GameOver`))
  ;[1 1 1] Game over
  (`WidgetLayoutLibrary.RemoveAllWidgets`)
  (`UserWidget.AddToViewport` _gameover 0)
  (`WidgetBlueprintLibrary.SetInputMode_UIOnlyEx` _returnvalue _gameover)
  (set `PlayerController.bShowMouseCursor` true _returnvalue)
  (`GameplayStatics.SetGamePaused` true))

(event `EventGanaste`
  (bind _returnvalue (`GameplayStatics.GetPlayerController` 0))
  (bind _ganaste (`self.Ganaste`))
  ;[1 1 1] Ganaste
  (`WidgetLayoutLibrary.RemoveAllWidgets`)
  (`UserWidget.AddToViewport` _ganaste 0)
  (`WidgetBlueprintLibrary.SetInputMode_UIOnlyEx` _returnvalue _ganaste)
  (set `PlayerController.bShowMouseCursor` true _returnvalue)
  (`GameplayStatics.SetGamePaused` true))

(event `self.ReceiveAnyDamage`
  (params (Damage :type "Float (single-precision)") (DamageType :type "DamageType Object Reference") (InstigatedBy :type "Controller Object Reference") (DamageCauser :type "Actor Object Reference"))
  ;[1 1 1] Deducir vida
  (`/Engine/EditorBlueprintResources/StandardMacros.DoOnce` false :!label _label
    (:`Completed`
      (bind _output_get (set `self.Vida` (- (`self.Vida`) Damage)))
      (if (<= _output_get 0.001)
        (`self.EventFinalDeJuego`)
        (else
          (set `self.MostrarDaño` true)
          (`KismetSystemLibrary.Delay` 0.3)
          (set `self.MostrarDaño` false)
          (`KismetSystemLibrary.Delay` 0.2)
          (goto _label :!via `Reset`))))))

(fn `UserConstructionScript`)