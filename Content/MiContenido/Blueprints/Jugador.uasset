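; Jugador is the player input Blueprint that drives the Personaje character and toggles the pause screen.
; On BeginPlay it casts player character 0 to Personaje and caches it.
; Input events forward jump, movement along the actor's forward and right vectors, and pitch/yaw look to that character.
; Pausa clears all widgets, flips game pause and shows the character's pause or HUD widget accordingly.
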(event `InputAction|Salto`
  (params (Key :type "Key Structure"))
  ;[1 1 1] Salto
  (:`Pressed`
    (`Character.Jump` (`self.Personaje`))))

(event `InputAxis|MovimientoAdelandeAtras`
  (params (AxisValue :type "Float (single-precision)"))
  (bind _personaje (`self.Personaje`))
  ;[1 1 1] Movimiento
  (`Pawn.AddMovementInput` _personaje (`self.GetActorForwardVector` _personaje) AxisValue false))

(event `InputAction|Pausa` :paused true
  (params (Key :type "Key Structure"))
  (bind _personaje (`self.Personaje`))
  ;[1 1 1] Pausa
  (:`Pressed`
    (`WidgetLayoutLibrary.RemoveAllWidgets`)
    (if (`GameplayStatics.IsGamePaused`)
      (`UserWidget.AddToViewport` (`/Game/MiContenido/Blueprints/Personaje.MyHUD` _personaje) 0)
      (`GameplayStatics.SetGamePaused` false)
      (else
        (`UserWidget.AddToViewport` (`/Game/MiContenido/Blueprints/Personaje.Pausa` _personaje) 0)
        (`GameplayStatics.SetGamePaused` true)))))

(event `self.ReceiveBeginPlay`
  ;[1 1 1] Llamar al personaje
  (bind _aspersonaje (cast `/Game/MiContenido/Blueprints/Personaje` (`GameplayStatics.GetPlayerCharacter` 0)))
  (set `self.Personaje` _aspersonaje))

(event `InputAxis|MovimientoIzquierdaDerecha`
  (params (AxisValue :type "Float (single-precision)"))
  (bind _personaje (`self.Personaje`))
  ;[1 1 1] Movimiento
  (`Pawn.AddMovementInput` _personaje (`self.GetActorRightVector` _personaje) AxisValue false))

(event `InputAxis|MiraArribaAbajo`
  (params (AxisValue :type "Float (single-precision)"))
  ;[1 1 1] Mirar alrededor
  (`Pawn.AddControllerPitchInput` (`self.Personaje`) AxisValue))

(event `InputAxis|MiraDerechaIzquierda`
  (params (AxisValue :type "Float (single-precision)"))
  ;[1 1 1] Mirar alrededor
  (`Pawn.AddControllerYawInput` (`self.Personaje`) AxisValue))

(fn `UserConstructionScript`)