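; Puerta is an exit door that the player can open only after collecting all the orbs.
; Its collision overlap checks the Personaje's points, sets an on-screen prompt and enables the door's input only at the required score.
; Leaving the overlap clears the message and disables input.
; The Interactuar press runs once, playing the AbrirPuerta timeline to swing the actor's yaw from its starting rotation.
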(event `self.ReceiveBeginPlay`)

(event `InputAction|Interactuar`
  (params (Key :type "Key Structure"))
  (:`Pressed`
    (`/Engine/EditorBlueprintResources/StandardMacros.DoOnce` false
      (:`Completed`
        ;[1 1 1] Rotacion de puerta
        (bind _output_get (set `self.RotacionInicial` (`self.K2_GetActorRotation`)))
        (bind (_direction _rotacion) (`Timeline|AbrirPuerta`)
          (:`Update`
            (`self.K2_SetActorRotation` (`KismetMathLibrary.MakeRotator` (.roll _output_get) (.pitch _output_get) (- (.yaw _output_get) _rotacion)))))))))

(event `self.ColisionDePuerta.OnComponentBeginOverlap`
  (params (OverlappedComponent :type "PrimitiveComponent Object Reference") (OtherActor :type "Actor Object Reference") (OtherComp :type "PrimitiveComponent Object Reference") (OtherBodyIndex :type Integer) (bFromSweep :type Boolean) (SweepResult :type "HitResult Structure (by ref)"))
  ;[1 1 1] Habilitar y desabilitar
  (bind _aspersonaje (cast `/Game/MiContenido/Blueprints/Personaje` OtherActor))
  (if (== (`/Game/MiContenido/Blueprints/Personaje.Puntos` _aspersonaje) 13)
    ;[1 1 1] Terminar juego
    (set `/Game/MiContenido/Blueprints/Personaje.MensajeEnPantalla` "Oprime F para abrir la puerta" _aspersonaje)
    (`self.EnableInput` (`GameplayStatics.GetPlayerController` 0))
    (else
      (set `/Game/MiContenido/Blueprints/Personaje.MensajeEnPantalla` "Obten todos los orbes para salir" _aspersonaje))))

(event `self.ColisionDePuerta.OnComponentEndOverlap`
  (params (OverlappedComponent :type "PrimitiveComponent Object Reference") (OtherActor :type "Actor Object Reference") (OtherComp :type "PrimitiveComponent Object Reference") (OtherBodyIndex :type Integer))
  ;[1 1 1] Habilitar y desabilitar
  (bind _aspersonaje (cast `/Game/MiContenido/Blueprints/Personaje` OtherActor))
  (set `/Game/MiContenido/Blueprints/Personaje.MensajeEnPantalla` "" _aspersonaje)
  ;[1 1 1] Terminar juego
  (`self.DisableInput` (`GameplayStatics.GetPlayerController` 0)))

(fn `UserConstructionScript`)